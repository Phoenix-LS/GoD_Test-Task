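; BP_Building is a building actor that shows its name and current versus maximum point storage on a widget component.
; On BeginPlay it binds to its BalanceChanged dispatcher and fires it once.
; Each change constructs a fresh WBP_Interaction_Prompt with those values and assigns it to the component, rather than updating the existing one.
; The construction script applies the configurable building mesh; its storage limit check has an empty branch.
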(event Custom|Balance%20Changed_Event
  (bind _returnvalue (Game|ConstructObjectfromClass "/Game/Buildings/UI/WBP_Interaction_Prompt.WBP_Interaction_Prompt_C" self (Utilities|Text|ToText(Integer) (Variables|BuildingStats|GetCurrent%20Storage)) (Utilities|Text|ToText(Integer) (Variables|BuildingStats|GetMax%20Storage)) (Variables|BuildingStats|GetName%20of%20the%20Building)))
  (UserInterface|SetWidget (Variables|Default|GetAmount%20of%20points%20in%20actor) _returnvalue))

(event EventBeginPlay
  (EventDispatchers|BindEventtoBalanceChanged (delegate Custom|Balance%20Changed_Event))
  (Default|CallBalanceChanged))

(fn ConstructionScript
  (Components|StaticMesh|SetStaticMesh (Variables|Default|GetStaticMesh) (Variables|BuildingVisuals|GetBuilding%20Mesh))
  (if (< (Variables|BuildingStats|GetMax%20Storage) (Variables|BuildingStats|GetCurrent%20Storage))
    _))