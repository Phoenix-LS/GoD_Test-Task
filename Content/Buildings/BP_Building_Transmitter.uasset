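; Transmitter building that drains stored points from a Source building entering its ScanCollision overlap.
; A custom delayed, breakable loop moves one point per tick, paced by PointsPerSecond, until the Transmitter is full or the Source is empty, firing both buildings' balance events for widget updates.
; IsConnectedToSource locks draining to one Source; the IfNotFull dispatcher releases it when CanDrainMoreThenOneTime is set and storage has room.
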(event OnComponentBeginOverlap(ScanCollision)
  (params (OverlappedComponent :type Primitive%20Component%20Object%20Reference) (OtherActor :type Actor%20Object%20Reference) (OtherComp :type Primitive%20Component%20Object%20Reference) (OtherBodyIndex :type Integer) (bFromSweep :type Boolean) (SweepResult :type Hit%20Result%20Structure%20%28by%20ref%29))
  ;[1 1 1] Scanning an actors around Transmitter to find building to drain points
  (if (not (Variables|Default|GetIs%20Connected%20To%20Source?))
    (bind _asbp_building_source (Utilities|Casting|CastToBP_Building_Source OtherActor))
    (Variables|Default|SetSource%20Building%20Ref _asbp_building_source)
    (Default|CallDrainStorage)
    (Development|PrintString (Utilities|String|ToString(Text) (Utilities|Text|FormatText "Its a {object}" OtherActor)))))

(event Custom|Event%20Drain%20Storage
  (bind _current_storage (Variables|Default|GetCurrent%20Storage))
  (bind _source_building_ref (Variables|Default|GetSource%20Building%20Ref))
  (bind _current_storage_2 (Variables|/Game/Buildings/BP_Building.BP_Building_C|GetCurrent%20Storage _source_building_ref))
  ;[1 1 1] Event to drain points from Source building
  (Variables|Default|SetIs%20Connected%20To%20Source? true) ; Locking drain process only on one building so it cannot be interrupted
  (bind _output_get (Variables|Default|SetTotal%20Storage%20Of%20a%20Target _current_storage_2))
  (Utilities|ForEachLoopwithBreakandDelay 0 (- _output_get 1) (Variables|Default|GetPoints%20Per%20Second) :!label _label
    (:Loop%20Body
      (if (and (!= (Variables|Default|GetCurrent%20Storage) (Variables|Default|GetMax%20Storage)) (!= _current_storage_2 0)) ; Is storage is full? And is there any points left in a target?
        (Math|Integer|IncrementInt _current_storage ; Adding points to our Storage
          (:%20%20
            (Math|Integer|DecrementInt (Variables|/Game/Buildings/BP_Building.BP_Building_C|GetCurrent%20Storage _source_building_ref) ; Removing points from Source
              (:%20%20
                (CallFunction|BalanceChangedEvent) ; Balance change event for real-time uploading results to the widget
                (Default|BalanceChangedEvent _source_building_ref)
                (Development|PrintString (Utilities|String|ToString(Integer) _current_storage)) ; Countdown
              ))))
        (else
          (Default|CallIfNotFull)
          (goto _label Break))))
    (:Completed
      (Development|PrintString (Utilities|String|ToString(Integer) _current_storage_2)) ; Debug for points left in a Source
      (Default|CallIfNotFull) ; If not full and it can drain more reseting the rule for draining lock
    )))

(event Custom|If%20not%20Full%20Event
  ;[1 1 1] Reseting lock rule if enabled
  (if (Variables|Default|GetCan%20Drain%20More%20Then%20One%20Time?)
    (if (< (Variables|Default|GetCurrent%20Storage) (Variables|Default|GetMax%20Storage))
      (Variables|Default|SetIs%20Connected%20To%20Source? false))))

(event EventBeginPlay
  (EventDispatchers|BindEventtoDrainStorage (delegate Custom|Event%20Drain%20Storage))
  (CallFunction|BalanceChangedEvent)
  (EventDispatchers|BindEventtoIfNotFull (delegate Custom|If%20not%20Full%20Event)))

(fn ConstructionScript
  (|CallParentFunction))